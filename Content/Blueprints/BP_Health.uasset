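; BP_Health is a health component that tracks damage taken by its owning actor.
; On BeginPlay it binds to the owner's OnTakeAnyDamage event, then subtracts each hit from CurrentHealth, clamped between zero and MaxHealth.
; When health is zero after a hit it calls DeathMessage on the owner, with no guard against repeat calls from later hits.
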(event Custom|TakeDamage
  (params (DamagedActor :type Actor%20Object%20Reference) (Damage :type Float%20%28single-precision%29) (DamageType :type Damage%20Type%20Object%20Reference) (InstigatedBy :type Controller%20Object%20Reference) (DamageCauser :type Actor%20Object%20Reference))
  (bind _output_get (Variables|Default|SetCurrentHealth (Math|Float|Clamp(Float) (- (Variables|Default|GetCurrentHealth) Damage) 0.0 (Variables|Default|GetMaxHealth))))
  (if (== _output_get 0.0)
    (Class|BPITakingDamage|Death(Message) (Components|GetOwner))))

(event EventBeginPlay
  (EventDispatchers|BindEventtoOnTakeAnyDamage (Components|GetOwner) (delegate Custom|TakeDamage)))