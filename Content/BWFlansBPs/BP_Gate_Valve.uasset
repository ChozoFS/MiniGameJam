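; Sliding door Blueprint that works as an interactable gate or as a valve that shuts when the player enters its trigger.
; A timeline lerps the moving mesh sideways, and Interact toggles it.
; Unless SimpleDoor is set, which only makes the meshes block, BeginPlay caches the player and opens non-Gate doors.
; With Valve set, player overlap closes an open door, using a box sized and placed in the construction script.
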(event OnComponentBeginOverlap(Box)
  (params (OverlappedComponent :type Primitive%20Component%20Object%20Reference) (OtherActor :type Actor%20Object%20Reference) (OtherComp :type Primitive%20Component%20Object%20Reference) (OtherBodyIndex :type Integer) (bFromSweep :type Boolean) (SweepResult :type Hit%20Result%20Structure%20%28by%20ref%29))
  (if (Math|Boolean|ANDBoolean (== OtherActor (Variables|Default|GetPlayerBP)) (Variables|Default|GetValve?) (Variables|Default|GetOpen?))
    (CallFunction|Close)))

(event Custom|Open
  (Variables|Default|SetOpen? true)
  (bind _dooralpha (Timeline|DoorTL PlayFromStart)
    (:Update
      (Transformation|SetRelativeLocation (Variables|Default|GetMovePieceSM) (Math|Vector|Lerp(Vector) "0, 0,125.000000" "0,130.000000,125.000000" _dooralpha) false false))))

(event Custom|Close
  (Variables|Default|SetOpen? false)
  (bind _dooralpha (Timeline|DoorTL ReverseFromEnd)
    (:Update
      (Transformation|SetRelativeLocation (Variables|Default|GetMovePieceSM) (Math|Vector|Lerp(Vector) "0, 0,125.000000" "0,130.000000,125.000000" _dooralpha) false false))))

(event EventBeginPlay
  (if (Variables|Default|GetSimpleDoor?)
    (Collision|SetCollisionResponsetoAllChannels (Variables|Default|GetStaticMesh) "ECR_Block")
    (else
      (bind _outactors (Actor|GetAllActorsOfClass "/Game/FirstPersonBP/Blueprints/FirstPersonCharacter.FirstPersonCharacter_C"))
      (Variables|Default|SetPlayerBP (Utilities|Array|Get(acopy) _outactors))
      (if (not (Variables|Default|GetGate?))
        (CallFunction|Open)))))

(event Collision|EventActorBeginOverlap
  (params (OtherActor :type Actor%20Object%20Reference)))

(event EventTick
  (params (DeltaSeconds :type Float%20%28single-precision%29)))

(fn ConstructionScript
  (bind _box (Variables|Default|GetBox))
  (Transformation|SetRelativeLocation _box (Variables|Default|GetValveBoxLocation) false false)
  (Components|Box|SetBoxExtent _box (Variables|Default|GetValveBoxShape) true))

(fn Interact
  (if (Variables|Default|GetOpen?)
    (CallFunction|Close)
    (else
      (CallFunction|Open)))
  (return "" 0.0))