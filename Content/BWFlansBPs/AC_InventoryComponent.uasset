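; Inventory component that tracks crafting materials, visor batteries, pistol ammo and carried weight, and owns the WB_Inventory widget.
; Pickups are matched by item name, storing unit weight; each count change updates encumbrance and pushes to the widget.
; Crafting converts materials into ammo or batteries without checking stock, while reloading moves reserve ammo into the clip.
; The widget is created collapsed at BeginPlay and toggled with the mouse cursor.
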(event Custom|-Leather
  (params (Delta :type Integer))
  (bind _wb_inventoryui (Variables|Default|GetWB_InventoryUI))
  (if (>= (- (Variables|Default|GetLeather) Delta) 0)
    (bind _output_get (Variables|Default|SetLeather (- (Variables|Default|GetLeather) Delta)))
    (Default|UpdateLeatherSlot _wb_inventoryui _output_get (* _output_get (Variables|Default|GetLeatherWeight)))
    (bind _output_get_2 (Variables|Default|SetCurEncumberance (- (Variables|Default|GetCurEncumberance) (Variables|Default|GetLeatherWeight))))
    (Default|UpdateCurrentWeight _wb_inventoryui _output_get_2)))

(event Custom|ToggleInvUI
  (bind _wb_inventoryui (Variables|Default|GetWB_InventoryUI))
  (if (Variables|Default|GetInvOpen?)
    (Widget|SetVisibility _wb_inventoryui "Collapsed")
    (Variables|Default|SetInvOpen? false)
    (CallFunction|ToggleMouseCursor)
    (else
      (Widget|SetVisibility _wb_inventoryui "Visible")
      (Variables|Default|SetInvOpen? true)
      (CallFunction|ToggleMouseCursor)
      (Default|UpdateMaxWeight (Variables|Default|GetWB_InventoryUI) (Variables|Default|GetMaxEncumberance)))))

(event Custom|-Cloth
  (params (Delta :type Integer))
  (bind _wb_inventoryui (Variables|Default|GetWB_InventoryUI))
  (if (>= (- (Variables|Default|GetCloth) Delta) 0)
    (bind _output_get (Variables|Default|SetCloth (- (Variables|Default|GetCloth) Delta)))
    (Default|UpdateClothSlot _wb_inventoryui _output_get (* _output_get (Variables|Default|GetClothWeight)))
    (bind _output_get_2 (Variables|Default|SetCurEncumberance (- (Variables|Default|GetCurEncumberance) (Variables|Default|GetClothWeight))))
    (Default|UpdateCurrentWeight _wb_inventoryui _output_get_2)))

(event Custom|CraftVisorBattery
  (bind _wb_inventoryui (Variables|Default|GetWB_InventoryUI))
  (bind _metalweight (Variables|Default|GetMetalWeight))
  (bind _leatherweight (Variables|Default|GetLeatherWeight))
  (bind _output_get (Variables|Default|SetMetal (- (Variables|Default|GetMetal) 2)))
  (bind _output_get_2 (Variables|Default|SetLeather (- (Variables|Default|GetLeather) 2)))
  (Variables|Default|SetVisorBatteries (+ (Variables|Default|GetVisorBatteries) 1))
  (Default|UpdateMetalSlot _wb_inventoryui _output_get (* _output_get _metalweight))
  (Default|UpdateLeatherSlot _wb_inventoryui _output_get_2 (* _output_get_2 _leatherweight))
  (bind _output_get_3 (Variables|Default|SetCurEncumberance (+ (Variables|Default|GetVisorBatteryWeight) (- (- (Variables|Default|GetCurEncumberance) (* _metalweight 2.0)) (* _leatherweight 2.0)))))
  (Default|UpdateCurrentWeight _wb_inventoryui _output_get_3)
  (Default|UpdateVisorBatteryTxt _wb_inventoryui (Variables|Default|GetVisorBatteries) (* (Variables|Default|GetVisorBatteries) (Variables|Default|GetVisorBatteryWeight))))

(event Custom|-Metal
  (params (Delta :type Integer))
  (bind _wb_inventoryui (Variables|Default|GetWB_InventoryUI))
  (if (>= (- (Variables|Default|GetMetal) Delta) 0)
    (bind _output_get (Variables|Default|SetMetal (- (Variables|Default|GetMetal) Delta)))
    (Default|UpdateMetalSlot _wb_inventoryui _output_get (* _output_get (Variables|Default|GetMetalWeight)))
    (bind _output_get_2 (Variables|Default|SetCurEncumberance (- (Variables|Default|GetCurEncumberance) (Variables|Default|GetMetalWeight))))
    (Default|UpdateCurrentWeight _wb_inventoryui _output_get_2)))

(event Custom|PickupItem
  (params (BaseItem :type BP%20Base%20Item%20Object%20Reference))
  (bind _wood (Variables|Default|GetWood))
  (bind _cloth (Variables|Default|GetCloth))
  (bind _leather (Variables|Default|GetLeather))
  (bind _metal (Variables|Default|GetMetal))
  (bind _wb_inventoryui (Variables|Default|GetWB_InventoryUI))
  (bind _visorbatteries (Variables|Default|GetVisorBatteries))
  (bind _wb_inventoryui_2 (Variables|Default|GetWB_InventoryUI))
  (bind _itemweight (Variables|/Game/BWFlansBPs/BP_BaseItem.BP_BaseItem_C|GetItemWeight BaseItem))
  (if (Utilities|Enum|Equal(Enum) (Variables|/Game/BWFlansBPs/BP_BaseItem.BP_BaseItem_C|GetItemName BaseItem) (Utilities|Text|ToText(String) "Wood"))
    (Variables|Default|SetWoodWeight _itemweight)
    (Development|PrintString "Picked up Wood")
    (bind _result (Math|Integer|IncrementInt _wood)
      (:%20%20
        (Default|UpdateWoodSlot _wb_inventoryui_2 _result (* _wood (Variables|Default|GetWoodWeight)))
        (bind _output_get (Variables|Default|SetCurEncumberance (+ (Variables|Default|GetCurEncumberance) (Variables|Default|GetWoodWeight))))
        (Default|UpdateCurrentWeight _wb_inventoryui _output_get)))
    (elif (Utilities|Enum|Equal(Enum) (Variables|/Game/BWFlansBPs/BP_BaseItem.BP_BaseItem_C|GetItemName BaseItem) (Utilities|Text|ToText(String) "Cloth"))
      (Variables|Default|SetClothWeight _itemweight)
      (bind _result_2 (Math|Integer|IncrementInt _cloth)
        (:%20%20
          (Default|UpdateClothSlot _wb_inventoryui_2 _result_2 (* _cloth (Variables|Default|GetClothWeight)))
          (bind _output_get_2 (Variables|Default|SetCurEncumberance (+ (Variables|Default|GetCurEncumberance) (Variables|Default|GetClothWeight))))
          (Default|UpdateCurrentWeight _wb_inventoryui _output_get_2)))
      (elif (Utilities|Enum|Equal(Enum) (Variables|/Game/BWFlansBPs/BP_BaseItem.BP_BaseItem_C|GetItemName BaseItem) (Utilities|Text|ToText(String) "Leather"))
        (Variables|Default|SetLeatherWeight _itemweight)
        (bind _result_3 (Math|Integer|IncrementInt _leather)
          (:%20%20
            (Default|UpdateLeatherSlot _wb_inventoryui_2 _result_3 (* _leather (Variables|Default|GetLeatherWeight)))
            (bind _output_get_3 (Variables|Default|SetCurEncumberance (+ (Variables|Default|GetCurEncumberance) (Variables|Default|GetLeatherWeight))))
            (Default|UpdateCurrentWeight _wb_inventoryui _output_get_3)))
        (elif (Utilities|Enum|Equal(Enum) (Variables|/Game/BWFlansBPs/BP_BaseItem.BP_BaseItem_C|GetItemName BaseItem) (Utilities|Text|ToText(String) "Metal"))
          (Variables|Default|SetMetalWeight _itemweight)
          (bind _result_4 (Math|Integer|IncrementInt _metal)
            (:%20%20
              (Default|UpdateMetalSlot _wb_inventoryui_2 _result_4 (* _metal (Variables|Default|GetMetalWeight)))
              (bind _output_get_4 (Variables|Default|SetCurEncumberance (+ (Variables|Default|GetCurEncumberance) (Variables|Default|GetMetalWeight))))
              (Default|UpdateCurrentWeight _wb_inventoryui _output_get_4)))
          (elif (Utilities|Enum|Equal(Enum) (Variables|/Game/BWFlansBPs/BP_BaseItem.BP_BaseItem_C|GetItemName BaseItem) (Utilities|Text|ToText(String) "Visor Battery"))
            (bind _output_get_5 (Variables|Default|SetVisorBatteryWeight _itemweight))
            (bind _result_5 (Math|Integer|IncrementInt _visorbatteries)
              (:%20%20
                (Default|UpdateVisorBatteryTxt _wb_inventoryui_2 _result_5 (* _visorbatteries _output_get_5))
                (bind _output_get_6 (Variables|Default|SetCurEncumberance (+ (Variables|Default|GetCurEncumberance) (Variables|Default|GetVisorBatteryWeight))))
                (Default|UpdateCurrentWeight _wb_inventoryui _output_get_6)))))))))

(event Custom|CraftPistolAmmo
  (bind _wb_inventoryui (Variables|Default|GetWB_InventoryUI))
  (bind _metalweight (Variables|Default|GetMetalWeight))
  (bind _woodweight (Variables|Default|GetWoodWeight))
  (bind _clothweight (Variables|Default|GetClothWeight))
  (bind _result (Math|Integer|DecrementInt (Variables|Default|GetMetal))
    (:%20%20
      (bind _result_2 (Math|Integer|DecrementInt (Variables|Default|GetCloth))
        (:%20%20
          (bind _result_3 (Math|Integer|DecrementInt (Variables|Default|GetWood))
            (:%20%20
              (Variables|Default|SetPistolAmmo (+ (Variables|Default|GetPistolAmmo) 24))
              (Default|UpdateMetalSlot _wb_inventoryui _result (* _result _metalweight))
              (Default|UpdateClothSlot _wb_inventoryui _result_2 (* _result_2 _clothweight))
              (Default|UpdateWoodSlot _wb_inventoryui _result_3 (* _result_3 _woodweight))
              (bind _output_get (Variables|Default|SetCurEncumberance (- (- (- (Variables|Default|GetCurEncumberance) _metalweight) _clothweight) _woodweight)))
              (Default|UpdateCurrentWeight _wb_inventoryui _output_get)
              (Default|UpdatePistolAmmo _wb_inventoryui (Variables|Default|GetPistolAmmo))
              (Default|UpdateInvAmmo (Variables|/Game/FirstPersonBP/Blueprints/FirstPersonCharacter.FirstPersonCharacter_C|GetHUD (Variables|Default|GetPlayerBP)) (Variables|Default|GetPistolAmmo)))))))))

(event Custom|-Wood
  (params (Delta :type Integer))
  (bind _wb_inventoryui (Variables|Default|GetWB_InventoryUI))
  (if (>= (- (Variables|Default|GetWood) Delta) 0)
    (bind _output_get (Variables|Default|SetWood (- (Variables|Default|GetWood) Delta)))
    (Default|UpdateWoodSlot _wb_inventoryui _output_get (* _output_get (Variables|Default|GetWoodWeight)))
    (bind _output_get_2 (Variables|Default|SetCurEncumberance (- (Variables|Default|GetCurEncumberance) (Variables|Default|GetWoodWeight))))
    (Default|UpdateCurrentWeight _wb_inventoryui _output_get_2)))

(event Custom|ToggleMouseCursor
  (bind _returnvalue (Game|GetPlayerController 0))
  (if (Variables|/Script/Engine.PlayerController|GetbShowMouseCursor _returnvalue)
    (Variables|/Script/Engine.PlayerController|SetbShowMouseCursor (Game|GetPlayerController 0) false)
    (else
      (Variables|/Script/Engine.PlayerController|SetbShowMouseCursor _returnvalue true))))

(event Custom|UseBattery
  (params (Delta :type Integer))
  (bind _wb_inventoryui (Variables|Default|GetWB_InventoryUI))
  (if (>= (- (Variables|Default|GetVisorBatteries) Delta) 0)
    (bind _output_get (Variables|Default|SetVisorBatteries (- (Variables|Default|GetVisorBatteries) Delta)))
    (Default|UpdateVisorBatteryTxt _wb_inventoryui _output_get (* _output_get (Variables|Default|GetVisorBatteryWeight)))
    (bind _output_get_2 (Variables|Default|SetCurEncumberance (- (Variables|Default|GetCurEncumberance) (Variables|Default|GetVisorBatteryWeight))))
    (Default|UpdateCurrentWeight _wb_inventoryui _output_get_2)))

(event Custom|DecrementClipAmmo
  (bind _result (Math|Integer|DecrementInt (Variables|Default|GetClipAmmo))
    (:%20%20
      (Development|PrintString (Utilities|String|Append "Clip ammo :" (Utilities|String|ToString(Integer) _result))))))

(event Custom|ReloadAmmo
  (bind _maxclipammo (Variables|Default|GetMaxClipAmmo))
  (if (< (- (Variables|Default|GetPistolAmmo) (- _maxclipammo (Variables|Default|GetClipAmmo))) 0)
    (Variables|Default|SetClipAmmo (+ (Variables|Default|GetClipAmmo) (Variables|Default|GetPistolAmmo)))
    (Variables|Default|SetPistolAmmo 0)
    (else
      (bind _output_get (Variables|Default|SetPistolAmmo (- (Variables|Default|GetPistolAmmo) (- _maxclipammo (Variables|Default|GetClipAmmo)))))
      (bind _output_get_2 (Variables|Default|SetClipAmmo _maxclipammo))
      (Development|PrintString (Utilities|String|Append "Clip ammo :" (Utilities|String|ToString(Integer) _output_get_2) "Inv Ammo : " (Utilities|String|ToString(Integer) _output_get))))))

(event EventBeginPlay
  (bind _returnvalue (UserInterface|CreateWidget "/Game/BWFlansBPs/WB_Inventory.WB_Inventory_C"))
  (bind _output_get (Variables|Default|SetWB_InventoryUI _returnvalue))
  (UserInterface|Viewport|AddtoViewport _output_get 0)
  (Widget|SetVisibility _output_get "Collapsed")
  (Variables|Default|SetInvOpen? false)
  (bind _outactors (Actor|GetAllActorsOfClass "/Game/FirstPersonBP/Blueprints/FirstPersonCharacter.FirstPersonCharacter_C"))
  (Variables|Default|SetPlayerBP (Utilities|Array|Get(acopy) _outactors)))

(event EventTick
  (params (DeltaSeconds :type Float%20%28single-precision%29)))