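; BP_CraftingTable is an interactable crafting station that opens a crafting widget for the player.
; BeginPlay creates the hidden widget and caches the FirstPersonCharacter, whose box overlap toggles a text prompt and CanInteract.
; Interact closes any open inventory, disables player input, shows the cursor and widget, and passes in the player's material counts.
; Highlight reveals a point light, which a Tick countdown hides again; CloseCraftingTable is an empty stub.
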(event OnComponentBeginOverlap(Box)
  (params (OverlappedComponent :type Primitive%20Component%20Object%20Reference) (OtherActor :type Actor%20Object%20Reference) (OtherComp :type Primitive%20Component%20Object%20Reference) (OtherBodyIndex :type Integer) (bFromSweep :type Boolean) (SweepResult :type Hit%20Result%20Structure%20%28by%20ref%29))
  (if (== OtherActor (Variables|Default|GetPlayerBP))
    (Development|SetHiddeninGame (Variables|Default|GetTextRender) false false)
    (Variables|Default|SetCanInteract true)))

(event OnComponentEndOverlap(Box)
  (params (OverlappedComponent :type Primitive%20Component%20Object%20Reference) (OtherActor :type Actor%20Object%20Reference) (OtherComp :type Primitive%20Component%20Object%20Reference) (OtherBodyIndex :type Integer))
  (if (== OtherActor (Variables|Default|GetPlayerBP))
    (Development|SetHiddeninGame (Variables|Default|GetTextRender) true false)
    (Variables|Default|SetCanInteract false)))

(event Custom|CloseCraftingTable)

(event EventBeginPlay
  (bind _returnvalue (UserInterface|CreateWidget "/Game/BWFlansBPs/WB_CraftingTable.WB_CraftingTable_C"))
  (Variables|Default|SetWBCraftingTable _returnvalue)
  (UserInterface|Viewport|AddtoViewport _returnvalue 0)
  (Widget|SetVisibility _returnvalue "Collapsed")
  (Variables|Default|SetWidgetOpen false)
  (bind _outactors (Actor|GetAllActorsOfClass "/Game/FirstPersonBP/Blueprints/FirstPersonCharacter.FirstPersonCharacter_C"))
  (Variables|Default|SetPlayerBP (Utilities|Array|Get(acopy) _outactors)))

(event Collision|EventActorBeginOverlap
  (params (OtherActor :type Actor%20Object%20Reference)))

(event EventTick
  (params (DeltaSeconds :type Float%20%28single-precision%29))
  (bind _output_get (Variables|Default|SetHighlightTimer (- (Variables|Default|GetHighlightTimer) DeltaSeconds)))
  (if (<= _output_get 0.0)
    (Development|SetHiddeninGame (Variables|Default|GetPointLight) true false)))

(event EventHighlight
  (Development|SetHiddeninGame (Variables|Default|GetPointLight) false false)
  (Variables|Default|SetHighlightTimer 5.0))

(fn ConstructionScript)

(fn Interact
  (bind _wbcraftingtable (Variables|Default|GetWBCraftingTable))
  (bind _playerbp (Variables|Default|GetPlayerBP))
  (bind _ac_inventorycomponent (Variables|/Game/FirstPersonBP/Blueprints/FirstPersonCharacter.FirstPersonCharacter_C|GetAC_InventoryComponent _playerbp))
  (if (Variables|Default|GetCanInteract)
    (if (Variables|/Game/BWFlansBPs/AC_InventoryComponent.AC_InventoryComponent_C|GetInvOpen? _ac_inventorycomponent)
      (Default|ToggleInvUI _ac_inventorycomponent))
    (Input|DisableInput _playerbp 0)
    (Widget|SetVisibility _wbcraftingtable "Visible")
    (Default|UpdateTableInventory _wbcraftingtable (Variables|/Game/BWFlansBPs/AC_InventoryComponent.AC_InventoryComponent_C|GetCloth _ac_inventorycomponent) (Variables|/Game/BWFlansBPs/AC_InventoryComponent.AC_InventoryComponent_C|GetMetal _ac_inventorycomponent) (Variables|/Game/BWFlansBPs/AC_InventoryComponent.AC_InventoryComponent_C|GetLeather _ac_inventorycomponent) (Variables|/Game/BWFlansBPs/AC_InventoryComponent.AC_InventoryComponent_C|GetWood _ac_inventorycomponent))
    (Variables|/Script/Engine.PlayerController|SetbShowMouseCursor (Game|GetPlayerController 0) true)))