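; BP_Lever is an interactable lever that toggles between pulled and unpulled and signals linked actors.
; Interact calls PullLever, which flips Pulled and plays or reverses the LeverAlpha timeline to rotate Arrow.
; The timeline sends InteractMessage to every LinkedActor on each update, not once per pull.
; Highlight shows a SpotLight, which Tick hides again when a ten-second countdown expires.
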(event Custom|PullLever
  (if (Variables|Default|GetPulled?)
    (Variables|Default|SetPulled? false)
    (bind _newtrack_0 (Timeline|LeverAlpha ReverseFromEnd)
      (:Update
        (Transformation|SetRelativeRotation (Variables|Default|GetArrow) (Math|Rotator|Lerp(Rotator) "30.000000, 0, 0" "-30.000000, 0, 0" _newtrack_0) false false)
        (for _array_element (Variables|Default|GetLinkedActor)
          (Class|BPIInteract|Interact(Message) _array_element))))
    (else
      (Variables|Default|SetPulled? true)
      (Timeline|LeverAlpha PlayFromStart))))

(event EventBeginPlay)

(event Collision|EventActorBeginOverlap
  (params (OtherActor :type Actor%20Object%20Reference)))

(event EventTick
  (params (DeltaSeconds :type Float%20%28single-precision%29))
  (bind _output_get (Variables|Default|SetHighlightTimer (- (Variables|Default|GetHighlightTimer) DeltaSeconds)))
  (if (<= _output_get 0.0)
    (Development|SetHiddeninGame (Variables|Default|GetSpotLight) true false)))

(event EventHighlight
  (Development|SetHiddeninGame (Variables|Default|GetSpotLight) false false)
  (Variables|Default|SetHighlightTimer 1e+01))

(fn ConstructionScript)

(fn Interact
  (CallFunction|PullLever)
  (return "" 0.0))