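; Base pickup item that the player can highlight and collect into their inventory.
; BeginPlay caches the first FirstPersonCharacter; Highlight shows a PointLight, which Tick hides when its ten-second timer runs out.
; Interact checks the player's encumbrance limit, then moves the item far below the player instead of destroying it.
; It then passes itself to the ACInventoryComponent and returns its name and weight.
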(event EventBeginPlay
  (bind _outactors (Actor|GetAllActorsOfClass "/Game/FirstPersonBP/Blueprints/FirstPersonCharacter.FirstPersonCharacter_C"))
  (Variables|Default|SetPlayerBP (Utilities|Array|Get(acopy) _outactors)))

(event Collision|EventActorBeginOverlap
  (params (OtherActor :type Actor%20Object%20Reference)))

(event EventTick
  (params (DeltaSeconds :type Float%20%28single-precision%29))
  (bind _output_get (Variables|Default|SetHighlightTimer (- (Variables|Default|GetHighlightTimer) DeltaSeconds)))
  (if (<= _output_get 0.0)
    (Development|SetHiddeninGame (Variables|Default|GetPointLight) true false)))

(event EventHighlight
  (Development|SetHiddeninGame (Variables|Default|GetPointLight) false false)
  (Variables|Default|SetHighlightTimer 1e+01))

(fn ConstructionScript)

(fn Interact
  (bind _playerbp (Variables|Default|GetPlayerBP))
  (bind _ac_inventorycomponent (Variables|/Game/FirstPersonBP/Blueprints/FirstPersonCharacter.FirstPersonCharacter_C|GetAC_InventoryComponent _playerbp))
  (if (not (> (+ (Variables|/Game/BWFlansBPs/AC_InventoryComponent.AC_InventoryComponent_C|GetCurEncumberance _ac_inventorycomponent) (Variables|Default|GetItemWeight)) (Variables|/Game/BWFlansBPs/AC_InventoryComponent.AC_InventoryComponent_C|GetMaxEncumberance _ac_inventorycomponent)))
    (Transformation|SetWorldLocation (Variables|Default|GetDefaultSceneRoot) (- (Transformation|GetActorLocation (Variables|Default|GetPlayerBP)) "0.000000, 0,1000.000000") false false)
    (Default|PickupItem (Variables|/Game/FirstPersonBP/Blueprints/FirstPersonCharacter.FirstPersonCharacter_C|GetAC_InventoryComponent (Variables|Default|GetPlayerBP)) self)
    (return (Variables|Default|GetItemName) (Variables|Default|GetItemWeight))))